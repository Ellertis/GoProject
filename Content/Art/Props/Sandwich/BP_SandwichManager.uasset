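; BP_SandwichManager adds and removes a row of BP_Sandwich props, tracking them in an array and a counter.
; AddSandwich plays a pop sound, spawns a sandwich at an offset step along the line from Start toward End, and animates its scale with a timeline.
; RemoveSandwich animates the last sandwich's scale with a second timeline, then destroys it, drops it from the array and decrements the counter.
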(event Custom|AddSandwich
  (bind _start (Variables|Default|GetStart))
  (bind _returnvalue (Transformation|GetActorLocation _start))
  (Audio|PlaySound2D "/Game/Audio/Gameplay/Sandwich/SandwichPickup/SandwichPopCue.SandwichPopCue" 1.0 1.0 0.0 0 0)
  (bind _result (Math|Integer|IncrementInt (Variables|Default|GetSandwichCounter))
    (:%20%20
      (bind _returnvalue_2 (Game|SpawnActorfromClass "/Game/Gameplay/Tile/BP_Sandwich.BP_Sandwich_C" (Math|Transform|MakeTransform (+ (* (- _result 1) (Variables|Default|GetOffset) (Math|Vector|GetUnitDirection(Vector) _returnvalue (Transformation|GetActorLocation (Variables|Default|GetEnd)))) _returnvalue) (Variables|Default|GetSandwichRotation) (Variables|Default|GetSandichh%20Scale)) "Undefined" "MultiplyWithRoot" 0 1.0 true 0))
      (Utilities|Array|Add (Variables|Default|GetSandwiches) _returnvalue_2)
      (bind _newtrack_0 (Timeline|Timeline PlayFromStart)
        (:Update
          (Transformation|SetActorScale3D _returnvalue_2 (Math|Conversions|ToVector(Float) _newtrack_0)))))))

(event Custom|RemoveSandwich
  (bind _sandwiches (Variables|Default|GetSandwiches))
  (bind _returnvalue (Utilities|Array|Length _sandwiches))
  (bind _returnvalue_2 (- _returnvalue 1))
  (bind _output (Utilities|Array|Get(acopy) _sandwiches _returnvalue_2))
  (bind _newtrack_0 (Timeline|Timeline_0 PlayFromStart)
    (:Update
      (Transformation|SetActorScale3D _output (Math|Conversions|ToVector(Float) _newtrack_0)))
    (:Finished
      (Actor|DestroyActor _output)
      (Utilities|Array|RemoveIndex _sandwiches _returnvalue_2)
      (Math|Integer|DecrementInt (Variables|Default|GetSandwichCounter)))))

(event EventBeginPlay)

(fn ConstructionScript)