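; BP_Sandwich is a sandwich prop that bobs up and down around its placed location.
; On BeginPlay it stores its start location and starts a looping timer that drives the vertical movement in place of Tick.
; Each movement step advances time by the timer interval and offsets Z with a sine wave scaled by speed and height variables.
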(event Custom|VerticalMovement
  (bind _actorstartlocation (Variables|Default|GetActorStartLocation))
  (bind _output_get (Variables|Default|SetTime (+ (Variables|Default|GetTimerTime) (Variables|Default|GetTime))))
  (Transformation|SetActorLocation (Math|Vector|MakeVector (.x _actorstartlocation) (.y _actorstartlocation) (+ (.z _actorstartlocation) (* (Math|Trig|Sin(Radians) (* _output_get (Variables|Default|GetSpeed))) (Variables|Default|GetHeight)))) false false))

(event EventBeginPlay
  (Variables|Default|SetActorStartLocation (Transformation|GetActorLocation))
  (bind _returnvalue (Utilities|Time|SetTimerbyEvent (EventDispatchers|CreateEvent :!event Custom|VerticalMovement) (Variables|Default|GetTimerTime) true true))
  (Variables|Default|SetVerticalTimer _returnvalue))

(fn ConstructionScript)