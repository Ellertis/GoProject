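; Snowman character Blueprint made of body and arm meshes, with selectable face and top-mesh variations.
; The construction script applies the chosen eye material and top mesh, and attaches a Niagara component to the left arm.
; ProcessAnim bobs the three body parts vertically with staggered delays through UpdateTimeAndLocation's lerps on a shared time counter.
; That animation is dormant: BeginPlay calls an empty LaucnhAnim, and the timer and level sequence setups are disconnected.
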(event Custom|LaucnhAnim)

(event Custom|ProcessAnim
  (CallFunction|UpdateTimeandLocation (Variables|Default|GetSM_Snowman_Bottom_a) 0.0 5e+01 (Variables|Default|GetIintialHeightBottom))
  (CallFunction|UpdateTimeandLocation (Variables|Default|GetSM_Snowman_Mid_a) 0.25 5e+01 (Variables|Default|GetIintialHeightMid))
  (CallFunction|UpdateTimeandLocation (Variables|Default|GetSM_Snowman_Top_a) 0.5 5e+01 (Variables|Default|GetIintialHeightTop)))

(event EventBeginPlay
  (CallFunction|LaucnhAnim))

(fn ConstructionScript
  (Transformation|AttachComponentToComponent (Variables|Default|GetNewNiagaraSystem) (Variables|Default|GetSM_Snowman_Arm_L_a) "None" "KeepRelative" "KeepWorld" "KeepRelative" true)
  (switch Utilities|FlowControl|Switch|SwitchonE_SnowmanVariationYeux (Variables|Default|GetVariation%20Yeux)
    (:NewEnumerator0
      (Rendering|Material|SetMaterial (Variables|Default|GetSM_Snowman_Top_a) 1 "/Game/Art/Chara/Snowmen/Material/MI_Snowman_Happy.MI_Snowman_Happy"))
    (:NewEnumerator1
      (Rendering|Material|SetMaterial (Variables|Default|GetSM_Snowman_Top_a) 1 "/Game/Art/Chara/Snowmen/Material/MI_Snowman_Frown.MI_Snowman_Frown"))
    (:NewEnumerator2
      _))
  (switch Utilities|FlowControl|Switch|SwitchonE_SnowmanVariationMesh (Variables|Default|GetVariation%20Mesh%20)
    (:NewEnumerator0
      (Components|StaticMesh|SetStaticMesh (Variables|Default|GetSM_Snowman_Top_a) "/Game/Art/Chara/Snowmen/Mesh/SM_Snowman_Top_a.SM_Snowman_Top_a"))))

(fn UpdateTimeandLocation
  (params (StaticMeshComponent :type Static%20Mesh%20Component%20Object%20Reference) (Delay :type Float%20%28double-precision%29) (ZOffset :type Float%20%28double-precision%29) (IntialHeight :type Float%20%28double-precision%29))
  (bind _relativelocation (Variables|/Script/Engine.SceneComponent|GetRelativeLocation StaticMeshComponent))
  (bind _relativelocation_2 (Variables|/Script/Engine.SceneComponent|GetRelativeLocation StaticMeshComponent))
  (if (<= Delay (Variables|Default|GetCurrAnimTime))
    (if (<= (Variables|Default|GetCurrAnimTime) (Variables|Default|GetAnimDuration))
      (Variables|Default|SetCurrAnimTime (+ (Utilities|Time|GetWorldDeltaSeconds) (Variables|Default|GetCurrAnimTime)))
      (Transformation|SetRelativeLocation StaticMeshComponent (Math|Vector|MakeVector (.x _relativelocation) (.y _relativelocation) (Math|Float|Lerp IntialHeight (+ IntialHeight ZOffset) (/ (- (Variables|Default|GetCurrAnimTime) Delay) (Variables|Default|GetAnimDuration)))) false false)
      (elif (<= (Variables|Default|GetCurrAnimTime) (* (Variables|Default|GetAnimDuration) 2.0))
        (Transformation|SetRelativeLocation StaticMeshComponent (Math|Vector|MakeVector (.x _relativelocation_2) (.y _relativelocation_2) (Math|Float|Lerp (+ IntialHeight ZOffset) IntialHeight (/ (- (Variables|Default|GetCurrAnimTime) Delay) (* (Variables|Default|GetAnimDuration) 2.0)))) false false)
        (Variables|Default|SetCurrAnimTime (+ (Utilities|Time|GetWorldDeltaSeconds) (Variables|Default|GetCurrAnimTime)))
        (else
          (Utilities|Time|PauseTimerbyHandle (Variables|Default|GetAnimTimer)))))
    (else
      (Variables|Default|SetCurrAnimTime (+ (Utilities|Time|GetWorldDeltaSeconds) (Variables|Default|GetCurrAnimTime))))))