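; BP_Gunter1 is the Gunter character art Blueprint, showing three damage stages through eye materials and brain components.
; The Construction Script switches on GunterState to set the skeletal mesh's eye material and toggle BrainStage1 and BrainStage2 visibility, attaching the brain for stages 1 and 2.
; UpdateGunterState stores the new state, but its switch has no actions, so visuals change only in the Construction Script.
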(event Custom|UpdateGunterState
  (params (NewGunterState :type E_GunterState%20Enum :default "NewEnumerator0"))
  (bind _output_get (Variables|Default|SetGunterState NewGunterState))
  (switch Utilities|FlowControl|Switch|SwitchonE_GunterState _output_get))

(fn ConstructionScript
  (bind _skeletalmesh (Variables|Default|GetSkeletalMesh))
  (switch Utilities|FlowControl|Switch|SwitchonE_GunterState (Variables|Default|GetGunterState)
    (:NewEnumerator0
      (Rendering|Material|SetMaterial _skeletalmesh 1 "/Game/Art/Chara/Gunter/Material/MI_Gunter_NoDamage_Eyes.MI_Gunter_NoDamage_Eyes")
      (Rendering|SetVisibility (Variables|Default|GetBrain%20stage%201) false false)
      (Rendering|SetVisibility (Variables|Default|GetBrain%20Stage%202) false false))
    (:NewEnumerator1
      (Rendering|Material|SetMaterial _skeletalmesh 1 "/Game/Art/Chara/Gunter/Material/MI_Gunter_1Damage_Eyes.MI_Gunter_1Damage_Eyes")
      (Transformation|AttachComponentToComponent (Variables|Default|GetBrain%20stage%201) 0 "None" "KeepRelative" "KeepRelative" "KeepRelative" true)
      (CallFunction|UpdateGunterState (Variables|Default|GetGunterState))
      (Rendering|SetVisibility (Variables|Default|GetBrain%20stage%201) true false)
      (Rendering|SetVisibility (Variables|Default|GetBrain%20Stage%202) false false))
    (:NewEnumerator2
      (Rendering|Material|SetMaterial _skeletalmesh 1 "/Game/Art/Chara/Gunter/Material/MI_Gunter_2Damage_Eyes.MI_Gunter_2Damage_Eyes")
      (Transformation|AttachComponentToComponent (Variables|Default|GetBrain%20Stage%202) 0 "None" "KeepRelative" "KeepRelative" "KeepRelative" true)
      (CallFunction|UpdateGunterState (Variables|Default|GetGunterState))
      (Rendering|SetVisibility (Variables|Default|GetBrain%20stage%201) false false)
      (Rendering|SetVisibility (Variables|Default|GetBrain%20Stage%202) true false))))