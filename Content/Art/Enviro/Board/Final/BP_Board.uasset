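; Game board actor with clickable sandwich, reset and exit buttons, plus Gunter's face and hearts, mostly inert in main-menu mode.
; Buttons animate via level sequences bound at runtime; the sandwich toggles the player's Jake placement mode, with a glowing lever driven by a looping timeline.
; Gunter's damage events swap the face texture and hide hearts.
; Finished reset animation closes the tiles and top before reloading the level; exit opens the pause menu.
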(event OnClicked(Board_Button_Sandwich)
  (params (TouchedComponent :type Primitive%20Component%20Object%20Reference) (ButtonPressed :type Key%20Structure :default "None"))
  (if (not (Variables|Default|GetMainMenu))
    (bind _asbp_go_pawn_player (Utilities|Casting|CastToBP_GoPawnPlayer (Game|Player|GetPlayerPawn 0)))
    (Class|GoPawnPlayer|ToggleJakePlacementMode _asbp_go_pawn_player)))

(event OnClicked(Board_Button_ResetLevel)
  (params (TouchedComponent :type Primitive%20Component%20Object%20Reference) (ButtonPressed :type Key%20Structure :default "None"))
  (if (not (Variables|Default|GetMainMenu))
    (Audio|PlaySound2D "/Game/Audio/UI/ButtonPressed/Button_Proto1_Cue.Button_Proto1_Cue" 1.0 1.0 0.0 0 0)
    (Sequencer|Player|Play (Variables|Default|GetLSP_BoardReset) :!class /Script/MovieScene.MovieSceneSequencePlayer)))

(event OnClicked(Board_Button_ExitGame)
  (params (TouchedComponent :type Primitive%20Component%20Object%20Reference) (ButtonPressed :type Key%20Structure :default "None"))
  (if (not (Variables|Default|GetMainMenu))
    (Audio|PlaySound2D "/Game/Audio/UI/ButtonPressed/Button_Proto1_Cue.Button_Proto1_Cue" 1.0 1.0 0.0 0 0)
    (Sequencer|Player|Play (Variables|Default|GetLSP_BoardExit) :!class /Script/MovieScene.MovieSceneSequencePlayer)))

(event Custom|GunterTookDamage
  (params (NewHP :type Integer))
  (bind _returnvalue (Utilities|Select :Index NewHP :Option%200 0 :Option%201 2 :Option%202 1))
  (Development|PrintString (Utilities|String|ToString(Integer) _returnvalue))
  (Rendering|Material|SetTextureParameterValue (Variables|Default|GetMID_Screen) "Texture" (Utilities|Array|Get(acopy) (Variables|Default|GetGunterTextures) _returnvalue))
  (switch int NewHP
    (:0
      (Development|SetHiddeninGame (Variables|Default|GetHearth) true false))
    (:1
      (Development|SetHiddeninGame (Variables|Default|GetHearth1) true false))
    (:2
      (Development|SetHiddeninGame (Variables|Default|GetHearth2) true false))))

(event Custom|GunterIsDead
  (params (EnemyRef :type Go%20Pawn%20Enemy%20Object%20Reference)))

(event Custom|TriggerDownAnim
  (if (not (Variables|Default|GetMainMenu))
    (Sequencer|Player|Stop (Variables|Default|GetLSP_BoardSandwichUp) :!class /Script/MovieScene.MovieSceneSequencePlayer)
    (Sequencer|Player|Play (Variables|Default|GetLSP_BoardSandwichDown) :!class /Script/MovieScene.MovieSceneSequencePlayer)))

(event Custom|TriggerNodSandwich
  (if (not (Variables|Default|GetMainMenu))
    (bind _asbp_go_pawn_player (Utilities|Casting|CastToBP_GoPawnPlayer (Game|Player|GetPlayerPawn 0)))
    (if (not (Variables|/Script/GoProject.GoPawnPlayer|GetbIsJakePlacementMode _asbp_go_pawn_player))
      (Sequencer|Player|Play (Variables|Default|GetLSP_BoardNodwich) :!class /Script/MovieScene.MovieSceneSequencePlayer))))

(event Custom|TriggerUpAnim
  (if (not (Variables|Default|GetMainMenu))
    (CallFunction|EndGlow)
    (Sequencer|Player|Stop (Variables|Default|GetLSP_BoardSandwichDown) :!class /Script/MovieScene.MovieSceneSequencePlayer)
    (Sequencer|Player|Play (Variables|Default|GetLSP_BoardSandwichUp) :!class /Script/MovieScene.MovieSceneSequencePlayer)))

(event Custom|LevierGlow
  (bind _newtrack_0 (Timeline|Glow PlayFromStart)
    (:Update
      (Rendering|Material|SetScalarParameterValue (Variables|Default|GetMID_Levier) "Brightness" _newtrack_0 :!class /Script/Engine.MaterialInstanceDynamic))
    (:Finished
      (Timeline|Glow PlayFromStart))))

(event Custom|ResetPressFinished
  (bind _returnvalue (Actor|GetActorOfClass "/Game/Gameplay/Tile/BP_TileManager.BP_TileManager_C"))
  (Utilities|IsValid _returnvalue
    (:Is%20Valid
      (Default|Close _returnvalue)
      (Utilities|FlowControl|Delay 0.4)
      (bind _returnvalue_2 (Actor|GetActorOfClass "/Game/Art/Enviro/Board/Final/BP_Top.BP_Top_C"))
      (Utilities|IsValid _returnvalue_2
        (:Is%20Valid
          (Default|BeginClosing _returnvalue_2)
          (EventDispatchers|BindEventtoClosingEnded _returnvalue_2 (delegate Custom|CustomEvent)))))))

(event Custom|EndGlow
  (Utilities|FlowControl|Sequence
    (:then_0
      (bind _newtrack_0 (Timeline|Glow Stop)
        (:Update
          (Rendering|Material|SetScalarParameterValue (Variables|Default|GetMID_Levier) "Brightness" _newtrack_0 :!class /Script/Engine.MaterialInstanceDynamic))
        (:Finished
          (Timeline|Glow PlayFromStart))))
    (:then_1
      (Rendering|Material|SetScalarParameterValueonMaterials (Variables|Default|GetBoard_Button_Sandwich) "Brightness" 1.0))))

(event Custom|CustomEvent
  (bind _returnvalue (Game|GetCurrentLevelName true))
  (Game|OpenLevel(byName) (Utilities|String|StringToName _returnvalue)))

(event Custom|ExitPressFinished
  (bind _foundwidgets (Widget|GetAllWidgetsOfClass "/Game/UI_Widget/WP_PauseMenu.WP_PauseMenu_C" true))
  (if (Utilities|Array|IsEmpty _foundwidgets)
    (bind _returnvalue (UserInterface|CreateWidget "/Game/UI_Widget/WP_PauseMenu.WP_PauseMenu_C"))
    (UserInterface|Viewport|AddtoViewport _returnvalue 0)))

(event EventBeginPlay
  (Audio|PlaySound2D "/Game/Audio/Ambient/BackgroundMusicCue.BackgroundMusicCue" 1.0 1.0 0.0 0 0)
  (if (not (Variables|Default|GetMainMenu))
    (bind (_outactor _returnvalue) (Sequencer|Player|CreateLevelSequencePlayer "/Game/Art/Enviro/Board/Final/BoardSandwich_Up.BoardSandwich_Up" (Utilities|Struct|MakeMovieSceneSequencePlaybackSettings false "(Value=0)" "(TickIntervalSeconds=0.000000,EvaluationBudgetMicroseconds=0.000000,bTickWhenPaused=False,bAllowRounding=True)" 1.0 0.0 false false false false false false "None" true)))
    (Class|LevelSequenceActor|AddBinding _outactor (|GetSequenceBinding) self false)
    (Variables|Default|SetLSP_BoardSandwichUp _returnvalue)
    (bind (_outactor_2 _returnvalue_2) (Sequencer|Player|CreateLevelSequencePlayer "/Game/Art/Enviro/Board/Final/BoardSandwich_Down.BoardSandwich_Down" (Utilities|Struct|MakeMovieSceneSequencePlaybackSettings false "(Value=0)" "(TickIntervalSeconds=0.000000,EvaluationBudgetMicroseconds=0.000000,bTickWhenPaused=False,bAllowRounding=True)" 1.0 0.0 false false false false false false "None" true)))
    (Class|LevelSequenceActor|AddBinding _outactor_2 (|GetSequenceBinding) self false)
    (Variables|Default|SetLSP_BoardSandwichDown _returnvalue_2)
    (bind (_outactor_3 _returnvalue_3) (Sequencer|Player|CreateLevelSequencePlayer "/Game/Art/Enviro/Board/Final/BoardSandwich_Nodwich.BoardSandwich_Nodwich" (Utilities|Struct|MakeMovieSceneSequencePlaybackSettings false "(Value=0)")))
    (Class|LevelSequenceActor|AddBinding _outactor_3 (|GetSequenceBinding) self false)
    (Variables|Default|SetLSP_BoardNodwich _returnvalue_3)
    (Utilities|FlowControl|DelayUntilNextTick)
    (bind _returnvalue_4 (Actor|GetActorOfClass "/Game/Gameplay/Enemies/BP_GoPawnEnemyGunter.BP_GoPawnEnemyGunter_C"))
    (Utilities|IsValid _returnvalue_4
      (:Is%20Valid
        (EventDispatchers|BindEventtoDamageTaken _returnvalue_4 (EventDispatchers|CreateEvent :!event Custom|GunterTookDamage))
        (EventDispatchers|BindEventtoOnEnemyDeath _returnvalue_4 (delegate Custom|GunterIsDead))
        (bind _returnvalue_5 (Rendering|Material|CreateDynamicMaterialInstance "/Game/Art/Material/Master/M_UnlitMasked.M_UnlitMasked" "None" "None" :!class /Script/Engine.KismetMaterialLibrary))
        (bind _output_get (Variables|Default|SetMID_Screen _returnvalue_5))
        (Rendering|Material|SetMaterial (Variables|Default|GetGunterFace) 0 _output_get)
        (Rendering|Material|SetTextureParameterValue _output_get "Texture" (Utilities|Array|Get(acopy) (Variables|Default|GetGunterTextures))))
      (:Is%20Not%20Valid
        _))
    (bind _returnvalue_6 (Rendering|Material|CreateDynamicMaterialInstance "/Game/Art/Enviro/Board/MI_Levier_Vrai.MI_Levier_Vrai" "None" "None" :!class /Script/Engine.KismetMaterialLibrary))
    (bind _output_get_2 (Variables|Default|SetMID_Levier _returnvalue_6))
    (Rendering|Material|SetMaterial (Variables|Default|GetBoard_Button_Sandwich) 1 _output_get_2)
    (bind (_outactor_4 _returnvalue_7) (Sequencer|Player|CreateLevelSequencePlayer "/Game/Art/Enviro/Board/Final/BoardReset.BoardReset" (Utilities|Struct|MakeMovieSceneSequencePlaybackSettings false "(Value=0)" "(TickIntervalSeconds=0.000000,EvaluationBudgetMicroseconds=0.000000,bTickWhenPaused=False,bAllowRounding=True)" 1.0 0.0 false false false false false false "None" true)))
    (Class|LevelSequenceActor|AddBinding _outactor_4 (|GetSequenceBinding) self false)
    (Variables|Default|SetLSP_BoardReset _returnvalue_7)
    (EventDispatchers|AssignOnFinished _returnvalue_7 (EventDispatchers|CreateEvent :!event Custom|ResetPressFinished))
    (bind (_outactor_5 _returnvalue_8) (Sequencer|Player|CreateLevelSequencePlayer "/Game/Art/Enviro/Board/Final/BoardExit.BoardExit" (Utilities|Struct|MakeMovieSceneSequencePlaybackSettings false "(Value=0)" "(TickIntervalSeconds=0.000000,EvaluationBudgetMicroseconds=0.000000,bTickWhenPaused=False,bAllowRounding=True)" 1.0 0.0 false false false false false false "None" true)))
    (Class|LevelSequenceActor|AddBinding _outactor_5 (|GetSequenceBinding) self false)
    (Variables|Default|SetLSP_BoardExit _returnvalue_8)
    (EventDispatchers|AssignOnFinished _returnvalue_8 (EventDispatchers|CreateEvent :!event Custom|ExitPressFinished))
    (else
      (Rendering|SetVisibility (Variables|Default|GetGunterFace) false false)
      (Rendering|SetVisibility (Variables|Default|GetHearth) false false)
      (Rendering|SetVisibility (Variables|Default|GetHearth1) false false)
      (Rendering|SetVisibility (Variables|Default|GetHearth2) false false))))

(event Collision|EventActorBeginOverlap
  (params (OtherActor :type Actor%20Object%20Reference)))

(event EventTick
  (params (DeltaSeconds :type Float%20%28single-precision%29)))

(fn ConstructionScript)