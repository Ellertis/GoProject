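; Game mode that runs a level's start, win and loss flow by binding to its game start, win and game over events.
; Start opens the BP_Top actor, and loss shows the lose screen.
; The first win records the finished level from the map name, saves, plays victory audio, shows the win screen, then closes the tile manager and top after delays.
; The WP_UI creation chain is disconnected.
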(event Custom|GameStarted
  (Variables|Default|SetWinCondition false)
  (bind _returnvalue (Actor|GetActorOfClass "/Game/Art/Enviro/Board/Final/BP_Top.BP_Top_C"))
  (Default|BeginOpening _returnvalue))

(event Custom|GameWon
  (bind _returnvalue (Game|GetGameInstance))
  (bind _returnvalue_2 (Game|GetPlayerController 0))
  (bind _asbp_game_instance (Utilities|Casting|CastToBP_GameInstance _returnvalue))
  (if (not (Variables|Default|GetWinCondition))
    (Variables|Default|SetWinCondition true)
    (bind _returnvalue_3 (Game|GetCurrentLevelName true))
    (Default|SetFinishedLevel _asbp_game_instance (Math|Integer|SelectInt 1 2 (Utilities|Enum|Equal(Enum) _returnvalue_3 "BasicMap2")))
    (Default|SaveGame _asbp_game_instance true)
    (Audio|PlaySound2D "/Game/Audio/Gameplay/Win/VictoryCue.VictoryCue" 1.0 1.0 0.0 0 0)
    (bind _returnvalue_4 (UserInterface|CreateWidget "/Game/UI_Widget/WP_WinScreen.WP_WinScreen_C" _returnvalue_2))
    (UserInterface|Viewport|AddtoViewport _returnvalue_4 0)
    (Input|SetInputModeUIOnly _returnvalue_2 _returnvalue_4 "DoNotLock" false)
    (Utilities|FlowControl|Delay 4.0)
    (bind _returnvalue_5 (Actor|GetActorOfClass "/Game/Gameplay/Tile/BP_TileManager.BP_TileManager_C"))
    (Utilities|IsValid _returnvalue_5
      (:Is%20Valid
        (Default|Close _returnvalue_5)
        (Utilities|FlowControl|Delay 0.4)
        (bind _returnvalue_6 (Actor|GetActorOfClass "/Game/Art/Enviro/Board/Final/BP_Top.BP_Top_C"))
        (Utilities|IsValid _returnvalue_6
          (:Is%20Valid
            (Default|BeginClosing _returnvalue_6)
            (EventDispatchers|BindEventtoClosingEnded _returnvalue_6 (delegate Custom|CustomEvent))))))))

(event Custom|GameLost
  (bind _returnvalue (Game|GetPlayerController 0))
  (bind _returnvalue_2 (UserInterface|CreateWidget "/Game/UI_Widget/WP_LoseScreenGunter.WP_LoseScreenGunter_C" _returnvalue))
  (UserInterface|Viewport|AddtoViewport _returnvalue_2 0)
  (Input|SetInputModeUIOnly _returnvalue _returnvalue_2 "DoNotLock" false))

(event Custom|CustomEvent)

(event EventBeginPlay
  (EventDispatchers|BindEventtoOnGameStart (EventDispatchers|CreateEvent :!event Custom|GameStarted))
  (EventDispatchers|BindEventtoOnGameWin (EventDispatchers|CreateEvent :!event Custom|GameWon))
  (EventDispatchers|BindEventtoOnGameOver (EventDispatchers|CreateEvent :!event Custom|GameLost)))

(fn ConstructionScript)