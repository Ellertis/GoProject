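; Game over screen actor that fades its Title component in and back out when play begins.
; Construction script assigns the base material to Title, and BeginPlay swaps in a dynamic instance with zero opacity.
; A single timeline drives the Fade_Opacity parameter, playing forward to fade in and, after a variable delay, in reverse to fade out.
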(event Custom|FadeIn
  (bind _opacity (Timeline|FadeInTimeLine PlayFromStart)
    (:Update
      (Rendering|Material|SetScalarParameterValue (Variables|Default|GetMID_Screen) "Fade_Opacity" _opacity :!class /Script/Engine.MaterialInstanceDynamic))))

(event Custom|FadeOut
  (bind _opacity (Timeline|FadeInTimeLine ReverseFromEnd)
    (:Update
      (Rendering|Material|SetScalarParameterValue (Variables|Default|GetMID_Screen) "Fade_Opacity" _opacity :!class /Script/Engine.MaterialInstanceDynamic))))

(event Custom|Trigger
  (CallFunction|Fadein)
  (Utilities|FlowControl|Delay (Variables|Default|GetDelay))
  (CallFunction|FadeOut))

(event EventBeginPlay
  (bind _returnvalue (Rendering|Material|CreateDynamicMaterialInstance (Variables|Default|GetMaterial) "None" "None" :!class /Script/Engine.KismetMaterialLibrary))
  (bind _output_get (Variables|Default|SetMID_Screen _returnvalue))
  (Rendering|Material|SetMaterial (Variables|Default|GetTitle) 0 _output_get)
  (Rendering|Material|SetScalarParameterValue (Variables|Default|GetMID_Screen) "Fade_Opacity" 0.0 :!class /Script/Engine.MaterialInstanceDynamic)
  (CallFunction|Trigger))

(fn ConstructionScript
  (Rendering|Material|SetMaterial (Variables|Default|GetTitle) 0 (Variables|Default|GetMaterial)))