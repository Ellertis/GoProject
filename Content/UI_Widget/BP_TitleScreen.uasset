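; Title screen Blueprint that shows the main menu logo and a press-any-key prompt, with fade in and fade out.
; On BeginPlay it creates dynamic material instances for the Title and PressAnyKey components and starts both fully transparent.
; FadeIn and FadeOut events play one timeline forward or in reverse, driving the Fade_Opacity parameter on both materials together.
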(event Custom|FadeIn
  (bind _opacity (Timeline|FadeInTimeLine PlayFromStart)
    (:Update
      (Rendering|Material|SetScalarParameterValue (Variables|Default|GetMID_Title) "Fade_Opacity" _opacity :!class /Script/Engine.MaterialInstanceDynamic)
      (Rendering|Material|SetScalarParameterValue (Variables|Default|GetMID_PressAnyKey) "Fade_Opacity" _opacity :!class /Script/Engine.MaterialInstanceDynamic))))

(event Custom|FadeOut
  (bind _opacity (Timeline|FadeInTimeLine ReverseFromEnd)
    (:Update
      (Rendering|Material|SetScalarParameterValue (Variables|Default|GetMID_Title) "Fade_Opacity" _opacity :!class /Script/Engine.MaterialInstanceDynamic)
      (Rendering|Material|SetScalarParameterValue (Variables|Default|GetMID_PressAnyKey) "Fade_Opacity" _opacity :!class /Script/Engine.MaterialInstanceDynamic))))

(event EventBeginPlay
  (bind _returnvalue (Rendering|Material|CreateDynamicMaterialInstance "/Game/UI_Widget/Textures/Title_Screen/Material/MI_MainMenuLogo.MI_MainMenuLogo" "None" "None" :!class /Script/Engine.KismetMaterialLibrary))
  (bind _output_get (Variables|Default|SetMID_Title _returnvalue))
  (Rendering|Material|SetMaterial (Variables|Default|GetTitle) 0 _output_get)
  (bind _returnvalue_2 (Rendering|Material|CreateDynamicMaterialInstance "/Game/UI_Widget/Textures/Title_Screen/Material/MI_PressPlay.MI_PressPlay" "None" "None" :!class /Script/Engine.KismetMaterialLibrary))
  (bind _output_get_2 (Variables|Default|SetMID_PressAnyKey _returnvalue_2))
  (Rendering|Material|SetMaterial (Variables|Default|GetPressAnyKey) 0 _output_get_2)
  (Rendering|Material|SetScalarParameterValue (Variables|Default|GetMID_Title) "Fade_Opacity" 0.0 :!class /Script/Engine.MaterialInstanceDynamic)
  (Rendering|Material|SetScalarParameterValue (Variables|Default|GetMID_PressAnyKey) "Fade_Opacity" 0.0 :!class /Script/Engine.MaterialInstanceDynamic))

(fn ConstructionScript)