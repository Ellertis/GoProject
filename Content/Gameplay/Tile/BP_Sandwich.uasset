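; BP_Sandwich is a collectible sandwich pickup that reports to BP_SandwichManager when collected.
; The player pawn's first overlap plays a PickUp level sequence bound to the actor, then adds a sandwich and destroys both actors.
; On BeginPlay, UI instances stay visible with rotation disabled, while others hide if tagged "Hide".
; A vertical bobbing event exists, but its timer setup is disconnected.
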(event OnComponentBeginOverlap(SM_Sandwich)
  (params (OverlappedComponent :type Primitive%20Component%20Object%20Reference) (OtherActor :type Actor%20Object%20Reference) (OtherComp :type Primitive%20Component%20Object%20Reference) (OtherBodyIndex :type Integer) (bFromSweep :type Boolean) (SweepResult :type Hit%20Result%20Structure%20%28by%20ref%29))
  (if (== OtherActor (Game|Player|GetPlayerPawn 0))
    (Utilities|FlowControl|DoOnce false
      (:Completed
        (bind (_outactor _returnvalue) (Sequencer|Player|CreateLevelSequencePlayer "/Game/Art/Props/Sandwich/PickUp.PickUp"))
        (Class|LevelSequenceActor|AddBinding _outactor (|GetSequenceBinding) self false)
        (Sequencer|Player|Play _returnvalue :!class /Script/MovieScene.MovieSceneSequencePlayer)
        (EventDispatchers|BindEventtoOnFinished _returnvalue (delegate Custom|CustomEvent))))))

(event Custom|VerticalMovement
  (if (or (>= (Variables|Default|GetCurrentTime) (Variables|Default|GetTimeLimit)) (<= (Variables|Default|GetCurrentTime) 0.0))
    (Variables|Default|SetTimerTime (* (Variables|Default|GetTimerTime) -1.0)))
  (Transformation|AddActorLocalOffset (Math|Vector|MakeVector 0.0 0.0 (Utilities|Operators|Divide (Variables|Default|GetTimeLimit) (Variables|Default|GetTimerTime) 3e+03)) false false)
  (Variables|Default|SetCurrentTime (Math|Float|Clamp(Float) (+ (Variables|Default|GetTimerTime) (Variables|Default|GetCurrentTime)) 0.0 (Variables|Default|GetTimeLimit))))

(event Custom|CustomEvent
  (bind _returnvalue (Actor|GetActorOfClass "/Game/Art/Props/Sandwich/BP_SandwichManager.BP_SandwichManager_C"))
  (Utilities|IsValid _returnvalue
    (:Is%20Valid
      (Default|AddSandwich _returnvalue))
    (:Is%20Not%20Valid
      _))
  (Actor|DestroyActor (stale OnComponentBeginOverlap(SM_Sandwich) _outactor))
  (Actor|DestroyActor))

(event EventBeginPlay
  (bind _rotatingmovement (Variables|Default|GetRotatingMovement))
  (if (Variables|Default|GetUI)
    (Rendering|SetActorHiddenInGame false)
    (Variables|/Script/Engine.RotatingMovementComponent|SetRotationRate _rotatingmovement "0, 0, 0")
    (Components|Activation|Deactivate _rotatingmovement)
    (else
      (Rendering|SetActorHiddenInGame (Actor|ActorHasTag "Hide")))))

(fn ConstructionScript)