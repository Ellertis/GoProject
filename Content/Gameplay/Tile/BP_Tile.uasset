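; Level tile actor that configures itself at BeginPlay from its TileType.
; After a one-tick delay, a switch makes Void tiles invisible via an invisible material, which Nothing/Un Jakeable tiles also apply to their debug mesh.
; Sandwich tiles spawn a half-scale SandwichRef actor at the tile's position, raised by SandwichOffset.
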(event EventBeginPlay
  (bind _returnvalue (Transformation|GetActorLocation))
  (Utilities|FlowControl|DelayUntilNextTick)
  (switch Utilities|FlowControl|Switch|SwitchonETileType (Variables|Default|GetTileType)
    (:Void
      (Rendering|Material|SetMaterial (Variables|Default|GetMeshComponent) 0 "/Game/Art/Material/Mesh/M_Invis.M_Invis"))
    (:Sandwich
      (Game|SpawnActorfromClass (Variables|Default|GetSandwichRef) (Math|Transform|MakeTransform (Math|Vector|MakeVector (.x _returnvalue) (.y _returnvalue) (+ (.z _returnvalue) (Variables|Default|GetSandwichOffset))) "0, 0, 0" "0.500000,0.500000,0.500000") "Undefined" "MultiplyWithRoot" 0 0))
    (:Nothing
      (Rendering|Material|SetMaterial (Variables|Default|GetMeshComponent) 0 "/Game/Art/Material/Mesh/M_Invis.M_Invis")
      (Rendering|Material|SetMaterial (Variables|Default|GetDebugMeshComponent) 0 "/Game/Art/Material/Mesh/M_Invis.M_Invis"))))

(event Collision|EventActorBeginOverlap
  (params (OtherActor :type Actor%20Object%20Reference)))

(event EventTick
  (params (DeltaSeconds :type Float%20%28single-precision%29)))

(fn ConstructionScript)