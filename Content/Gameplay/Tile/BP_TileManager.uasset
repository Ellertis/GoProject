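; Tile manager that animates two tagged groups of actors vertically for opening and closing sequences, after hiding them at BeginPlay.
; Opening and Close share one path; Close first inverts the offset and direction flag.
; When enabled, the path records each actor's Z, then staggers two timelines with delays, unhiding and lerping each group by the offset.
; Actors tagged Hide are revealed as the second group starts moving.
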(event Custom|InitialMoveTimeline2
  (for _array_element (Variables|Default|GetActorToMove2)
    (Rendering|SetActorHiddenInGame _array_element false))
  (bind _alpha (Timeline|MoveUpTimeline2 PlayFromStart)
    (:Update
      (for (_array_element_2 _array_index) (Variables|Default|GetActorToMove2)
        (Transformation|SetActorLocation _array_element_2 (Math|Vector|MakeVector (.x (Transformation|GetActorLocation _array_element_2)) (.y (Transformation|GetActorLocation _array_element_2)) (Math|Float|Lerp (Utilities|Array|Get(acopy) (Variables|Default|GetInitialActorsLocation2) _array_index) (+ (Utilities|Array|Get(acopy) (Variables|Default|GetInitialActorsLocation2) _array_index) (Variables|Default|GetInitialMoveOffset)) _alpha)) false false)))
    (:Finished
      (Utilities|Array|Clear (Variables|Default|GetActorToMove2))
      (Utilities|Array|Clear (Variables|Default|GetInitialActorsLocation2)))))

(event Custom|InitialMoveTimeline
  (for _array_element (Variables|Default|GetActorsToMove)
    (Rendering|SetActorHiddenInGame _array_element false))
  (bind _alpha (Timeline|MoveUpTimeline PlayFromStart)
    (:Update
      (for (_array_element_2 _array_index) (Variables|Default|GetActorsToMove)
        (Transformation|SetActorLocation _array_element_2 (Math|Vector|MakeVector (.x (Transformation|GetActorLocation _array_element_2)) (.y (Transformation|GetActorLocation _array_element_2)) (Math|Float|Lerp (Utilities|Array|Get(acopy) (Variables|Default|GetInitialActorsLocation) _array_index) (+ (Utilities|Array|Get(acopy) (Variables|Default|GetInitialActorsLocation) _array_index) (Variables|Default|GetInitialMoveOffset)) _alpha)) false false)))
    (:Finished
      (Utilities|Array|Clear (Variables|Default|GetActorsToMove))
      (Utilities|Array|Clear (Variables|Default|GetInitialActorsLocation)))))

(event Custom|Close
  (Variables|Default|SetInitialMoveOffset (* (Variables|Default|GetInitialMoveOffset) -1.0))
  (Variables|Default|SetUp/Down (not (Variables|Default|GetUp/Down)))
  (if (Variables|Default|GetTriggerInitialMove)
    (bind _outactors (Actor|GetAllActorswithTag "InitialMovement"))
    (bind _output_get (Variables|Default|SetActorsToMove _outactors))
    (if (Utilities|Array|IsNotEmpty _output_get)
      (Utilities|FlowControl|Delay (Variables|Default|GetFirstDelay))
      (for _array_element (Variables|Default|GetActorsToMove)
        (if (Variables|Default|GetUp/Down)
          (Transformation|AddActorLocalOffset _array_element (Math|Vector|MakeVector 0.0 0.0 (* (Variables|Default|GetInitialMoveOffset) -1.0)) false false)
          (else
            (Rendering|SetActorHiddenInGame true)))
        (Utilities|Array|Add (Variables|Default|GetInitialActorsLocation) (.z (Transformation|GetActorLocation _array_element))))
      (CallFunction|InitialMoveTimeline))
    (Utilities|FlowControl|Delay (Variables|Default|GetSecondDelay))
    (bind _outactors_2 (Actor|GetAllActorswithTag "InitialMovement2"))
    (bind _output_get_2 (Variables|Default|SetActorToMove2 _outactors_2))
    (if (Utilities|Array|IsNotEmpty _output_get_2)
      (for _array_element_2 (Variables|Default|GetActorToMove2)
        (if (Variables|Default|GetUp/Down)
          (Transformation|AddActorLocalOffset _array_element_2 (Math|Vector|MakeVector 0.0 0.0 (* (Variables|Default|GetInitialMoveOffset) -1.0)) false false))
        (Utilities|Array|Add (Variables|Default|GetInitialActorsLocation2) (.z (Transformation|GetActorLocation _array_element_2))))
      (CallFunction|InitialMoveTimeline2)
      (bind _outactors_3 (Actor|GetAllActorswithTag "Hide"))
      (for _array_element_3 _outactors_3
        (Rendering|SetActorHiddenInGame _array_element_3 false)))))

(event Custom|Opening
  (if (Variables|Default|GetTriggerInitialMove)
    (bind _outactors (Actor|GetAllActorswithTag "InitialMovement"))
    (bind _output_get (Variables|Default|SetActorsToMove _outactors))
    (if (Utilities|Array|IsNotEmpty _output_get)
      (Utilities|FlowControl|Delay (Variables|Default|GetFirstDelay))
      (for _array_element (Variables|Default|GetActorsToMove)
        (if (Variables|Default|GetUp/Down)
          (Transformation|AddActorLocalOffset _array_element (Math|Vector|MakeVector 0.0 0.0 (* (Variables|Default|GetInitialMoveOffset) -1.0)) false false)
          (else
            (Rendering|SetActorHiddenInGame true)))
        (Utilities|Array|Add (Variables|Default|GetInitialActorsLocation) (.z (Transformation|GetActorLocation _array_element))))
      (CallFunction|InitialMoveTimeline))
    (Utilities|FlowControl|Delay (Variables|Default|GetSecondDelay))
    (bind _outactors_2 (Actor|GetAllActorswithTag "InitialMovement2"))
    (bind _output_get_2 (Variables|Default|SetActorToMove2 _outactors_2))
    (if (Utilities|Array|IsNotEmpty _output_get_2)
      (for _array_element_2 (Variables|Default|GetActorToMove2)
        (if (Variables|Default|GetUp/Down)
          (Transformation|AddActorLocalOffset _array_element_2 (Math|Vector|MakeVector 0.0 0.0 (* (Variables|Default|GetInitialMoveOffset) -1.0)) false false))
        (Utilities|Array|Add (Variables|Default|GetInitialActorsLocation2) (.z (Transformation|GetActorLocation _array_element_2))))
      (CallFunction|InitialMoveTimeline2)
      (bind _outactors_3 (Actor|GetAllActorswithTag "Hide"))
      (for _array_element_3 _outactors_3
        (Rendering|SetActorHiddenInGame _array_element_3 false)))))

(event EventBeginPlay
  (Utilities|FlowControl|DelayUntilNextTick)
  (bind _outactors (Actor|GetAllActorswithTag "InitialMovement"))
  (bind _output_get (Variables|Default|SetActorsToMove _outactors))
  (if (Utilities|Array|IsNotEmpty _output_get)
    (for _array_element _output_get
      (Rendering|SetActorHiddenInGame _array_element true))
    (Utilities|Array|Clear (Variables|Default|GetActorsToMove))
    (bind _outactors_2 (Actor|GetAllActorswithTag "InitialMovement2"))
    (bind _output_get_2 (Variables|Default|SetActorToMove2 _outactors_2))
    (if (Utilities|Array|IsNotEmpty _output_get_2)
      (for _array_element_2 (Variables|Default|GetActorToMove2)
        (Rendering|SetActorHiddenInGame _array_element_2 true))
      (Utilities|Array|Clear (Variables|Default|GetActorToMove2)))))

(fn ConstructionScript)