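; BP_GoPawnEnemyGunter is the Gunter enemy pawn Blueprint, handling its visual feedback for movement, fear, fleeing and damage.
; Tick shows a billboard and runs a snow effect while fleeing.
; Movement and fear events call toggle functions, with a short delay before fear completion is signaled.
; Taking damage fires a snow impact and matches damage meshes and eye material to remaining Health.
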(event EventBeginPlay)

(event Collision|EventActorBeginOverlap
  (params (OtherActor :type Actor%20Object%20Reference)))

(event EventOnDeath)

(event EventOnMoveStart
  (Default|CallToggleMovement true))

(event EventOnMoveEnd
  (Default|CallToggleMovement false))

(event EventPlayFearAnimation
  (Default|CallToggleFear true)
  (Utilities|FlowControl|Delay 0.63)
  (Default|CallToggleFear false)
  (Class|GoPawnEnemyGunter|OnFearAnimationComplete))

(event EventTick
  (params (DeltaSeconds :type Float%20%28single-precision%29))
  (bind _snowrunstate (Variables|Default|GetSnowRunState))
  (bind _billboard (Variables|Default|GetBillboard))
  (if (Variables|Default|GetbIsFleeing)
    (Rendering|SetVisibility _billboard true false)
    (Components|Activation|Activate _snowrunstate false)
    (else
      (Rendering|SetVisibility _billboard false false)
      (Components|Activation|Deactivate _snowrunstate))))

(event EventOnDamageTaken
  (params (Amount :type Integer) (HitDirection :type EFaceDirection%20Enum :default "Xplus"))
  (bind _gunter (Variables|Default|GetGunter))
  (Components|Activation|Activate (Variables|Default|GetSnowImpact) true)
  (switch int (Variables|Default|GetHealth)
    (:1
      (Rendering|SetVisibility (Variables|Default|GetGunter_Chara_1Damage) false false)
      (Rendering|SetVisibility (Variables|Default|GetGunter_Chara_2Damage) true false)
      (Rendering|Material|SetMaterial _gunter 1 "/Game/Art/Chara/Gunter/Material/MI_Gunter_2Damage_Eyes.MI_Gunter_2Damage_Eyes"))
    (:2
      (Rendering|SetVisibility (Variables|Default|GetGunter_Chara_1Damage) true false)
      (Rendering|SetVisibility (Variables|Default|GetGunter_Chara_2Damage) false false)
      (Rendering|Material|SetMaterial _gunter 1 "/Game/Art/Chara/Gunter/Material/MI_Gunter_1Damage_Eyes.MI_Gunter_1Damage_Eyes"))
    (:3
      (Rendering|Material|SetMaterial (Variables|Default|GetGunter) 1 "/Game/Art/Chara/Gunter/Material/MI_Gunter_NoDamage_Eyes.MI_Gunter_NoDamage_Eyes"))))

(fn ConstructionScript)