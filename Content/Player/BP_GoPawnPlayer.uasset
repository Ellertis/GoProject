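; Player pawn for the board game, reacting to move, rotation, damage and Jake tile events, with damage triggering game over once.
; Placement mode swaps valid void tiles for preview Jake tiles; placing one spends a sandwich through the SandwichManager.
; Removing the Jake tile plays a runtime-bound level sequence, then destroys it.
; CheckLevier makes the board lever and valid tiles glow when placement is possible and sandwiches remain.
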(event Custom|CustomEvent
  (Actor|DestroyActor (Variables|Default|GetCurrentJakeTile))
  (Variables|Default|SetCurrentJakeTile 0)
  (Actor|DestroyActor (stale EventOnRemoveJakeTile _outactor)))

(event EventBeginPlay
  (bind _returnvalue (Actor|GetActorOfClass "/Game/Art/Props/Sandwich/BP_SandwichManager.BP_SandwichManager_C"))
  (Utilities|IsValid _returnvalue
    (:Is%20Valid
      (Variables|Default|SetSandwichManager _returnvalue))
    (:Is%20Not%20Valid
      _))
  (bind _returnvalue_2 (Actor|GetActorOfClass "/Game/Art/Enviro/Board/Final/BP_Board.BP_Board_C"))
  (Utilities|IsValid _returnvalue_2
    (:Is%20Valid
      (Variables|Default|SetBoardREF _returnvalue_2))
    (:Is%20Not%20Valid
      _))
  (bind _asbp_go_game_mode_base (Utilities|Casting|CastToBP_GoGameModeBase (Game|GetGameMode)))
  (Variables|Default|SetGameModeRef _asbp_go_game_mode_base))

(event Collision|EventActorBeginOverlap
  (params (OtherActor :type Actor%20Object%20Reference)))

(event EventOnRotationEnd
  (Default|CallToggleRotation false))

(event EventOnTryEnterJakePlacementMode
  (bind _boardref (Variables|Default|GetBoardREF))
  (Utilities|FlowControl|DelayUntilNextTick)
  (Utilities|IsValid _boardref
    (:Is%20Valid
      (Default|TriggerNodSandwich _boardref))))

(event EventOnMoveStart
  (Default|CallToggleMovement true)
  (Variables|Default|SetTempVoidTiles (Class|GoPawnPlayer|GetValidJakePlacementTiles)))

(event EventOnMoveEnd
  (bind _ns_snowimpact1 (Variables|Default|GetNS_SnowImpact1))
  (Default|CallToggleMovement false)
  (CallFunction|CheckLevier)
  (if (not (== (Variables|Default|GetCurrTile) (Variables|Default|GetCurrentJakeTile)))
    (Components|Activation|Activate _ns_snowimpact1 false)
    (Utilities|FlowControl|Delay 0.5)
    (Components|Activation|Deactivate _ns_snowimpact1)
    (CallFunction|CheckLevier)))

(event EventOnDamageTaken
  (Components|Activation|Activate (Variables|Default|GetSnowImpact) false)
  (if (not (Variables|Default|GetDamageTaken))
    (Variables|Default|SetDamageTaken true)
    (bind _asbp_go_game_mode_base (Utilities|Casting|CastToBP_GoGameModeBase (Game|GetGameMode)))
    (Class|GoGameModeBase|GameOver _asbp_go_game_mode_base)))

(event EventOnEnterJakePlacementMode
  (bind _boardref (Variables|Default|GetBoardREF))
  (Utilities|IsValid _boardref
    (:Is%20Valid
      (Default|TriggerUpAnim _boardref))
    (:Is%20Not%20Valid
      _))
  (Variables|Default|SetTempVoidTiles (Class|GoPawnPlayer|GetValidJakePlacementTiles))
  (for _array_element (Variables|Default|GetTempVoidTiles)
    (Rendering|SetVisibility (Variables|/Script/GoProject.GoTile|GetRoot _array_element) false true)
    (bind _returnvalue (Game|SpawnActorfromClass "/Game/Gameplay/Tile/BP_TileJake.BP_TileJake_C" (Math|Transform|MakeTransform (Transformation|GetActorLocation _array_element) "0, 0, 0" "1.000000,1.000000,1.000000") "Undefined" "MultiplyWithRoot" 0 0))
    (Default|PreviewSetup _returnvalue)
    (Utilities|Array|Add (Variables|Default|GetPreviewJakeTiles) _returnvalue)))

(event EventOnRotationStart
  (Default|CallToggleRotation true))

(event EventOnRemoveJakeTile
  (Components|Animation|PlayAnimation (Variables|Default|GetJake) "/Game/Art/Chara/Jake/JakeDown.JakeDown" false)
  (bind (_outactor _returnvalue) (Sequencer|Player|CreateLevelSequencePlayer "/Game/Art/Props/JakeTile/TileJakeDown.TileJakeDown"))
  (Class|LevelSequenceActor|AddBinding _outactor (|GetSequenceBinding) (Variables|Default|GetCurrentJakeTile) false)
  (Sequencer|Player|Play _returnvalue :!class /Script/MovieScene.MovieSceneSequencePlayer)
  (EventDispatchers|BindEventtoOnFinished _returnvalue (delegate Custom|CustomEvent)))

(event EventOnExitJakePlacementMode
  (bind _boardref (Variables|Default|GetBoardREF))
  (Utilities|IsValid _boardref
    (:Is%20Valid
      (Default|TriggerDownAnim _boardref)
      (CallFunction|CheckLevier))
    (:Is%20Not%20Valid
      _))
  (for _array_element (Variables|Default|GetTempVoidTiles)
    (Rendering|SetVisibility (Variables|/Script/GoProject.GoTile|GetRoot _array_element) true true))
  (for _array_element_2 (Variables|Default|GetPreviewJakeTiles)
    (Default|PreviewRemove _array_element_2))
  (Utilities|Array|Clear (Variables|Default|GetPreviewJakeTiles)))

(event EventOnPlaceJakeTile
  (bind _currentjaketile (Variables|Default|GetCurrentJakeTile))
  (bind _sandwichmanager (Variables|Default|GetSandwichManager))
  (Components|Animation|PlayAnimation (Variables|Default|GetJake) "/Game/Art/Chara/Jake/JakeUP.JakeUP" false)
  (Rendering|SetVisibility (Variables|/Script/GoProject.GoTile|GetRoot (Variables|Default|GetCurrentJakeTile)) false true)
  (Utilities|IsValid _sandwichmanager
    (:Is%20Valid
      (Default|RemoveSandwich _sandwichmanager))
    (:Is%20Not%20Valid
      _))
  (Utilities|FlowControl|Delay 0.1)
  (Rendering|SetVisibility (Variables|/Script/GoProject.GoTile|GetRoot _currentjaketile) true true)
  (bind _asbp_tile_jake (Utilities|Casting|CastToBP_TileJake _currentjaketile))
  (Default|TrueSetup _asbp_tile_jake))

(fn ConstructionScript)

(fn CheckLevier
  (Utilities|IsValid (Variables|Default|GetBoardREF)
    (:Is%20Valid
      (Default|EndGlow (Variables|Default|GetBoardREF))
      (for _array_element (Variables|Default|GetTempVoidTiles)
        (bind _asbp_tile (Utilities|Casting|CastToBP_Tile _array_element))
        (Default|EndGlow _asbp_tile))
      (if (and (> (Utilities|Array|Length (Class|GoPawnPlayer|GetValidJakePlacementTiles)) 0) (> (Class|GoGameModeBase|GetSandwichCount (Variables|Default|GetGameModeRef)) 0))
        (Default|LevierGlow (Variables|Default|GetBoardREF))
        (for _array_element_2 (Class|GoPawnPlayer|GetValidJakePlacementTiles)
          (bind _asbp_tile_2 (Utilities|Casting|CastToBP_Tile _array_element_2))
          (Default|TileGlow _asbp_tile_2))))))